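; Player controller that turns the controlled pawn to face the mouse cursor and handles player death.
; Each tick, while the game is started, unpaused and the Player_BP is alive, it sets the pawn's yaw toward a cursor trace hit.
; GameStart and PlayerDied event bindings drive its state: start enables aiming, while death disables pawn input, pauses the game and calls Restart.
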(event `self.ReceiveTick`
  (params (DeltaSeconds :type "Float (single-precision)"))
  (bind _returnvalue (`self.K2_GetPawn`))
  (bind (_returnvalue_roll _returnvalue_pitch _returnvalue_yaw) (`KismetMathLibrary.BreakRotator` (`KismetMathLibrary.FindLookAtRotation` (`self.K2_GetActorLocation` _returnvalue) (`.Location` (`GameplayStatics.BreakHitResult` (`self.GetHitResultUnderCursorByChannel` "TraceTypeQuery3"))))))
  (if (and (`self.GameStarted`) (not (`GameplayStatics.IsGamePaused`)))
    (bind _asplayer_bp (cast `/Game/Blueprints/Player_BP` _returnvalue))
    (if (`PlayerCharacter.bIsAlive` _asplayer_bp)
      (`self.K2_SetActorRotation` _returnvalue (`KismetMathLibrary.MakeRotator` 0.0 0.0 _returnvalue_yaw) false))))

(event `self.ReceiveBeginPlay`
  (add `self.GameStart` (delegate `GameStart_Event`))
  (add `self.PlayerDied` (delegate `PlayerDied_Event`)))

(event `PlayerDied_Event`
  (`self.DisableInput` (`self.K2_GetPawn`) self)
  (`GameplayStatics.SetGamePaused` true)
  (`self.Restart`))

(event `GameStart_Event`
  (set `self.GameStarted` true))

(fn `UserConstructionScript`)