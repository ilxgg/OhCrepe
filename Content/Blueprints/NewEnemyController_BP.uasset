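; Enemy AI controller that runs Enemy_BT on possession and feeds it player perception through the Blackboard.
; A successfully sensed Player-tagged actor cancels the timer and records line of sight, last location and actor reference.
; Any other perception update starts a looping delayed timer that re-polls sight.
; That check refreshes those keys or clears sight and reference, keeping the last known location.
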(event `self.ReceivePossess`
  (params (PossessedPawn :type "Pawn Object Reference"))
  (`self.RunBehaviorTree` "/Game/AI/Enemy_BT.Enemy_BT"))

(event `self.AIPerception.OnTargetPerceptionUpdated`
  (params (Actor :type "Actor Object Reference") (Stimulus :type "AIStimulus Structure"))
  (bind (_age _expirationage _strength _stimuluslocation _receiverlocation _tag _bsuccessfullysensed) (break `AIStimulus` Stimulus))
  (bind _blackboard (`self.Blackboard`))
  (if (and (`self.ActorHasTag` Actor "Player") _bsuccessfullysensed)
    (`KismetSystemLibrary.K2_ClearAndInvalidateTimerHandle` (`self.EnemyTimer`))
    (`BlackboardComponent.SetValueAsBool` _blackboard (`self.HasLineOfSight`) true)
    (`BlackboardComponent.SetValueAsVector` _blackboard (`self.PlayerLastLocation`) _stimuluslocation)
    (`BlackboardComponent.SetValueAsObject` _blackboard (`self.PlayerRef`) Actor)
    (`BlackboardComponent.SetValueAsBool` _blackboard (`self.JustCheckedLastLocation`) false)
    (else
      (bind _returnvalue (`KismetSystemLibrary.K2_SetTimerDelegate` (delegate `Start Enemy Timer`) (`self.LineOfSightTimer`) true))
      (set `self.EnemyTimer` _returnvalue))))

(event `Start Enemy Timer`
  (bind _blackboard (`self.Blackboard`))
  (bind _blackboard_2 (`self.Blackboard`))
  (set `self.PlayerInSight` false)
  (for _array_element (`AIPerceptionComponent.GetCurrentlyPerceivedActors` (`self.AIPerception`) "/Script/AIModule.AISense_Sight")
    (if (`self.ActorHasTag` _array_element "Player")
      (set `self.PlayerInSight` true)
      (`BlackboardComponent.SetValueAsBool` _blackboard_2 (`self.HasLineOfSight`) true)
      (`BlackboardComponent.SetValueAsVector` _blackboard_2 (`self.PlayerLastLocation`) (`self.K2_GetActorLocation` _array_element))
      (`BlackboardComponent.SetValueAsObject` _blackboard_2 (`self.PlayerRef`) _array_element)
      (`BlackboardComponent.SetValueAsBool` _blackboard_2 (`self.JustCheckedLastLocation`) false)))
  (if (not (`self.PlayerInSight`))
    (`BlackboardComponent.SetValueAsBool` _blackboard (`self.HasLineOfSight`) false)
    (`BlackboardComponent.SetValueAsObject` _blackboard (`self.PlayerRef`) null)))

(fn `UserConstructionScript`)