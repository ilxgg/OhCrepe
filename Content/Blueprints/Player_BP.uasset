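; Player Blueprint that connects the character's weapon, health and ammo state to its HUD.
; PlayerInit stores and shows the HUD, and both it and SwitchWeapon sync Knife and Ketchup visibility and the HUD weapon display to IsUsingMelee.
; Tick refreshes the magazine readout while not using melee.
; OnDamageTaken pushes health to the HUD and notifies PlayerController_BP when the player is no longer alive.
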(event `PlayerInit`
  (params (NewParam :type "/Game/UI/HUD_UI Object Reference"))
  (bind _bisusingmelee (`self.bIsUsingMelee`))
  (bind _output_get (set `self.HUDRef` NewParam))
  (`UserWidget.AddToViewport` _output_get 0)
  (`self.UpdateMag`)
  (`SceneComponent.SetVisibility` (`self.Knife`) _bisusingmelee false :!label _label)
  (`SceneComponent.SetVisibility` (`self.Ketchup`) (not _bisusingmelee) false)
  (`/Game/UI/HUD_UI.SwapWeapon` (`self.HUDRef`) _bisusingmelee))

(event `InputAction|SwitchWeapon` :overrideparent false
  (params (Key :type "Key Structure"))
  (:`Pressed`
    (goto _label)))

(event `self.OnDamageTaken`
  (`/Game/UI/HUD_UI.PlayerTakeDamage` (`self.HUDRef`) (`self.PlayerCurrentHealth`))
  (if (not (`self.bIsAlive`))
    (bind _asplayer_controller_bp (cast `/Game/Blueprints/PlayerController_BP` (`self.GetController`)))
    (`/Game/Blueprints/PlayerController_BP.PlayerDied` _asplayer_controller_bp)))

(event `self.ReceiveTick`
  (params (DeltaSeconds :type "Float (single-precision)"))
  (if (not (`self.bIsUsingMelee`))
    (`/Game/UI/HUD_UI.UpdateMagSize` (`self.HUDRef`) (`self.CurrentAmmoInMag`) (`self.MagSize`) :!label _label_2)))

(event `UpdateMag`
  (goto _label_2))

(fn `UserConstructionScript`)